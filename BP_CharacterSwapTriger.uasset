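; BP_CharacterSwapTriger is a trigger actor that lets player 0 switch control to another pawn while something overlaps it.
; Any actor beginning overlap enables the trigger's input, while ending overlap and BeginPlay disable it, with no check on which actor overlaps.
; Pressing E makes the player controller unpossess its current pawn, possess the PawnToPosess reference, then disables the trigger's input.
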(event `self.ReceiveActorEndOverlap`
  (params (OtherActor :type "Actor Object Reference"))
  (`self.DisableInput` (`GameplayStatics.GetPlayerController` 0) :!label _label))

(event `self.ReceiveBeginPlay`
  (goto _label))

(event `self.ReceiveActorBeginOverlap`
  (params (OtherActor :type "Actor Object Reference"))
  (`self.EnableInput` (`GameplayStatics.GetPlayerController` 0)))

(event `Key|E`
  (params (Key :type "Key Structure"))
  (bind _returnvalue (`GameplayStatics.GetPlayerController` 0))
  (:`Pressed`
    (`Controller.UnPossess` _returnvalue)
    (`Controller.Possess` _returnvalue (`self.PawnToPosess`))
    (`self.DisableInput` _returnvalue)))

(fn `UserConstructionScript`)